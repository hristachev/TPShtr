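; Third-person player character Blueprint with camera-relative movement, sprint, jump, toggle crouch, rifle equip and aiming.
; Equip and aim play montages only when none is running, while TakeRiffle reattaches the rifle between back and hand sockets.
; Aiming requires an equipped weapon and grounded state, changes speed, and interpolates capsule yaw toward control rotation on Tick.
; Timelines blend spring-arm framing for sprint and aim, and crouch events offset the boom against camera jerks.
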(event `RotationYawAim`
  (bind (_returnvalue_roll _returnvalue_pitch _returnvalue_yaw) (`KismetMathLibrary.BreakRotator` (`self.GetControlRotation`)))
  (bind _capsulecomponent (`self.CapsuleComponent`))
  (bind (_returnvalue_roll_2 _returnvalue_pitch_2) (`KismetMathLibrary.BreakRotator` (`SceneComponent.K2_GetComponentRotation` _capsulecomponent)))
  (if (`self.bIsAiming`)
    (`SceneComponent.K2_SetWorldRotation` (`self.CapsuleComponent`) (`KismetMathLibrary.RInterpTo` (`SceneComponent.K2_GetComponentRotation` _capsulecomponent) (`KismetMathLibrary.MakeRotator` _returnvalue_roll_2 _returnvalue_pitch_2 _returnvalue_yaw) (`GameplayStatics.GetWorldDeltaSeconds`) (`self.Interpolation Aiming Speed`)) false false)))

(event `self.ReceiveTick`
  (params (DeltaSeconds :type "Float (single-precision)"))
  (`|ExecutionSequence`
    (:`then_0`
      (`self.RotationYawAim`))))

(event `SprintingCameraOffsetStart`
  ;[1 0.3229 0.9942] Отдаление\Приближение камеры при спринте
  (if (not (`self.bIsAiming`))
    (bind (_direction _alpha_value) (`Timeline|Sprinting Offset` :!label _label)
      (:`Update`
        (set `SpringArmComponent.TargetArmLength` (`KismetMathLibrary.Lerp` 300.0 (`self.Sprinting Camera Arm Length`) _alpha_value) (`self.CameraBoom`))))))

(event `ToAim`
  (params (MontageToPlay :type "AnimMontage Object Reference"))
  (bind _charactermovement (`self.CharacterMovement`))
  ;[1 0 0] Прицеливание
  (if (`AnimInstance.IsAnyMontagePlaying` (`self.GetAnimInstance`))
    _
    (elif (`self.bIsWeaponEquipped`)
      (if (not (`NavMovementComponent.IsFalling` (`self.CharacterMovement`)))
        (`|ExecutionSequence`
          (:`then_0`
            (set `self.bIsAiming` true)
            (`AnimInstance.Montage_Play` (`self.GetAnimInstance`) MontageToPlay 1.0 "MontageLength" 0.0 true)
            (set `CharacterMovementComponent.bOrientRotationToMovement` false _charactermovement)
            (set `CharacterMovementComponent.MaxWalkSpeed` (`self.Aiming Speed`) _charactermovement))
          (:`then_1`
            (bind (_direction _arm_length_value) (`Timeline|CameraArmAiming` :!label _label_2)
              (:`Update`
                (set `SpringArmComponent.TargetArmLength` (`KismetMathLibrary.Lerp` (select `bool` (`self.bIsSprinting`) :`false` 300.0 :`true` (`self.Sprinting Camera Arm Length`)) 70.0 _arm_length_value) (`self.CameraBoom`))
                (set `SpringArmComponent.SocketOffset` (`KismetMathLibrary.MakeVector` 0.0 (`KismetMathLibrary.Lerp` 90.0 50.0 _arm_length_value) (`KismetMathLibrary.Lerp` 70.0 65.0 _arm_length_value)) (`self.CameraBoom`))))))))))

(event `ReverseCameraAiming`
  ;[1 0 0] Прицеливание
  (goto _label_2 :!via `Reverse`))

(event `SprintingCameraOffsetReverse`
  ;[1 0.3229 0.9942] Отдаление\Приближение камеры при спринте
  (if (not (`self.bIsAiming`))
    (goto _label :!via `Reverse`)))

(event `ToStopAim`
  (params (`Montage to Stop` :type "AnimMontage Object Reference"))
  ;[1 0 0] Прицеливание
  (`self.ReverseCameraAiming`)
  (set `self.bIsAiming` false)
  (set `CharacterMovementComponent.bOrientRotationToMovement` true (`self.CharacterMovement`))
  (`AnimInstance.Montage_Stop` (`self.GetAnimInstance`) 0.0 `Montage to Stop`)
  (set `CharacterMovementComponent.MaxWalkSpeed` (select `bool` (`self.bIsSprinting`) :`false` (`self.Run Speed`) :`true` (`self.Sprint Speed`)) (`self.CharacterMovement`)))

(event `InputAxis|Move Forward`
  (params (AxisValue :type "Float (single-precision)"))
  (bind (_returnvalue_roll _returnvalue_pitch _returnvalue_yaw) (`KismetMathLibrary.BreakRotator` (`self.GetControlRotation`)))
  ;[0.07087 1 0.6957 1 38] Axis Input's
  ;[1 1 1] Движение вперёд/назад
  (`self.AddMovementInput` (`KismetMathLibrary.GetForwardVector` (`KismetMathLibrary.MakeRotator` 0.0 0.0 _returnvalue_yaw)) AxisValue))

(event `InputAction|Sprint`
  (params (Key :type "Key Structure"))
  (bind _charactermovement (`self.CharacterMovement`))
  ;[1 0.3105 0.6202 1 38] Action input's
  ;;[1 1 1] Ускорение
  (:`Pressed`
    (if (not (`self.bIsAiming`))
      (`self.SetCrouch` false)
      (set `self.bIsSprinting` true)
      (set `CharacterMovementComponent.MaxWalkSpeed` (`self.Sprint Speed`) _charactermovement)
      (`self.SprintingCameraOffsetStart`)))
  (:`Released`
    (set `self.bIsSprinting` false)
    (set `CharacterMovementComponent.MaxWalkSpeed` (`self.Run Speed`) _charactermovement)
    (`self.SprintingCameraOffsetReverse`)))

(event `InputAxis|Move Right`
  (params (AxisValue :type "Float (single-precision)"))
  (bind (_returnvalue_roll _returnvalue_pitch _returnvalue_yaw) (`KismetMathLibrary.BreakRotator` (`self.GetControlRotation`)))
  ;[0.07087 1 0.6957 1 38] Axis Input's
  ;[1 1 1] Движение влево/вправо
  (`self.AddMovementInput` (`KismetMathLibrary.GetRightVector` (`KismetMathLibrary.MakeRotator` 0.0 0.0 _returnvalue_yaw)) AxisValue))

(event `InputAction|Jump`
  (params (Key :type "Key Structure"))
  ;[1 0.3105 0.6202 1 38] Action input's
  ;;[1 1 1] Прыжок
  (:`Pressed`
    (`self.Jump`))
  (:`Released`
    (`self.StopJumping`)))

(event `InputAxis|Look Right`
  (params (AxisValue :type "Float (single-precision)"))
  ;[0.07087 1 0.6957 1 38] Axis Input's
  ;[1 1 1] Движение камеры вправо/влево
  (`self.AddControllerYawInput` AxisValue))

(event `InputAction|Crouch`
  (params (Key :type "Key Structure"))
  ;[1 0.3105 0.6202 1 38] Action input's
  ;;[1 1 1] Присяд
  (:`Pressed`
    (`self.SetCrouch` (not (`self.bIsCrouching`)))))

(event `InputAxis|Look Up`
  (params (AxisValue :type "Float (single-precision)"))
  ;[0.07087 1 0.6957 1 38] Axis Input's
  ;[1 1 1] Движение камеры вверх/вниз
  (`self.AddControllerPitchInput` AxisValue))

(event `self.K2_OnStartCrouch`
  (params (HalfHeightAdjust :type "Float (single-precision)") (ScaledHalfHeightAdjust :type "Float (single-precision)"))
  ;[1 0.3105 0.6202 1 38] Action input's
  ;;[1 1 1] Присяд
  ;;;[0.8934 1 0.4631] Убираем дерганье камеры
  (set `SpringArmComponent.TargetOffset` (`KismetMathLibrary.MakeVector` 0.0 0.0 HalfHeightAdjust) (`self.CameraBoom`)))

(event `self.K2_OnEndCrouch`
  (params (HalfHeightAdjust :type "Float (single-precision)") (ScaledHalfHeightAdjust :type "Float (single-precision)"))
  ;[1 0.3105 0.6202 1 38] Action input's
  ;;[1 1 1] Присяд
  ;;;[0.8934 1 0.4631] Убираем дерганье камеры
  (set `SpringArmComponent.TargetOffset` (0.0 0.0 0.0) (`self.CameraBoom`)))

(event `InputAction|EquipUnequipWeapons`
  (params (Key :type "Key Structure"))
  ;[1 0.3105 0.6202 1 38] Action input's
  ;;[1 1 1] Экипировать\Убрать оружие
  (:`Pressed`
    (if (`AnimInstance.IsAnyMontagePlaying` (`self.GetAnimInstance`))
      _
      (elif (`self.bIsWeaponEquipped`)
        (set `self.bIsWeaponEquipped` false)
        (set `self.WeaponsType` "NewEnumerator0")
        (`AnimInstance.Montage_Play` (`self.GetAnimInstance`) "/Game/Animations/CharacterAnim/MainPlayer/AnimsWGuns/Rifle/Montage/AM_UnEquip_Rifle_Stand.AM_UnEquip_Rifle_Stand" 1.0 "MontageLength" 0.0 true)
        (else
          (set `self.bIsWeaponEquipped` true)
          (set `self.WeaponsType` "NewEnumerator1")
          (`AnimInstance.Montage_Play` (`self.GetAnimInstance`) "/Game/Animations/CharacterAnim/MainPlayer/AnimsWGuns/Rifle/Montage/AM_Equip_Rifle_Stand.AM_Equip_Rifle_Stand" 1.0 "MontageLength" 0.0 true))))))

(event `TakeRiffle`
  (params (bReturnWeapon :type Boolean))
  ;[1 0.3105 0.6202 1 38] Action input's
  ;;[1 1 1] Экипировать\Убрать оружие
  ;;;[0.404 1 0.9502] Взять\Убрать Оружие с привязкой к сокету
  (`SceneComponent.K2_AttachToComponent` (`self.RiffleBack`) (select `bool` bReturnWeapon :`false` (`self.WeaponSocketEquipHand`) :`true` (`self.WeaponSocketBack`)) "None" "KeepRelative" "KeepRelative" "KeepRelative" true))

(event `InputAction|Aiming`
  (params (Key :type "Key Structure"))
  ;[1 0.3105 0.6202 1 38] Action input's
  ;;[1 1 1] Прицеливание
  (:`Pressed`
    (`self.ToAim` "/Game/Animations/CharacterAnim/MainPlayer/AnimsWGuns/Rifle/Montage/AM_Idle_Rifle.AM_Idle_Rifle"))
  (:`Released`
    (`self.ToStopAim` "/Game/Animations/CharacterAnim/MainPlayer/AnimsWGuns/Rifle/Montage/AM_Idle_Rifle.AM_Idle_Rifle")))

(fn `GetAnimInstance`
  (returns (ReturnValue :type "AnimInstance Object Reference"))
  (return (`SkeletalMeshComponent.GetAnimInstance` (`self.Mesh`))))

(fn `SetCrouch`
  (params (`Is Crouch` :type Boolean))
  (bind _output_get (set `self.bIsCrouching` `Is Crouch`))
  (if _output_get
    (`self.Crouch`)
    (else
      (`self.UnCrouch`))))

(fn `UserConstructionScript`)